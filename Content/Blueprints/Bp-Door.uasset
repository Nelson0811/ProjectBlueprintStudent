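; Interactable double door Blueprint that swings two door meshes open and closed.
; BeginPlay caches each door's starting relative rotation as the base for the animation.
; Each Interact call toggles two FlipFlops that play or reverse separate Timelines, one per door.
; Timeline updates add yaw scaled by the Rotation variable, with a hardcoded offset subtracted from it for the second door.
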(event `self.ReceiveBeginPlay`
  (set `self.Relative Rotation` (`SceneComponent.RelativeRotation` (`self.Door_2`)))
  (set `self.Relative Rotation_0` (`SceneComponent.RelativeRotation` (`self.Door_1`))))

(event `/Game/Blueprints/interface/interface.interact`
  (bind (_relative_rotation_0_roll _relative_rotation_0_pitch _relative_rotation_0_yaw) (`KismetMathLibrary.BreakRotator` (`self.Relative Rotation_0`)))
  (bind (_relative_rotation_roll _relative_rotation_pitch _relative_rotation_yaw) (`KismetMathLibrary.BreakRotator` (`self.Relative Rotation`)))
  (`|ExecutionSequence`
    (:`then_0`
      (`/Engine/EditorBlueprintResources/StandardMacros.FlipFlop`
        (:`A`
          (bind (_direction _newtrack_0) (`Timeline|Timeline` :!label _label)
            (:`Update`
              (`SceneComponent.K2_SetRelativeRotation` (`self.Door_1`) (`KismetMathLibrary.MakeRotator` _relative_rotation_0_roll _relative_rotation_0_pitch (+ _relative_rotation_0_yaw (* _newtrack_0 (`self.Rotation`)))) false false))))
        (:`B`
          (goto _label :!via `Reverse`))))
    (:`then_1`
      (`/Engine/EditorBlueprintResources/StandardMacros.FlipFlop`
        (:`A`
          (bind (_direction_2 _newtrack_0_2) (`Timeline|Timeline_0` :!label _label_2)
            (:`Update`
              (`SceneComponent.K2_SetRelativeRotation` (`self.Door_2`) (`KismetMathLibrary.MakeRotator` _relative_rotation_roll _relative_rotation_pitch (+ _relative_rotation_yaw (* _newtrack_0_2 (- (`self.Rotation`) 150.0)))) false false))))
        (:`B`
          (goto _label_2 :!via `Reverse`))))))

(fn `UserConstructionScript`)